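; Interactable chest actor that opens and closes when interacted with.
; A box trigger shows a text prompt while the main character (BP_MainCH) overlaps it and hides it on exit.
; The Interact event toggles the ChestOpen flag and plays the matching open or close animation on the chest mesh.
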(event OnComponentBeginOverlap(Box)
  (params (OverlappedComponent :type Primitive%20Component%20Object%20Reference) (OtherActor :type Actor%20Object%20Reference) (OtherComp :type Primitive%20Component%20Object%20Reference) (OtherBodyIndex :type Integer) (bFromSweep :type Boolean) (SweepResult :type Hit%20Result%20Structure%20%28by%20ref%29))
  ;[1 1 1] Texto sobre cofre
  (Utilities|Casting|CastToBP_MainCH OtherActor)
  (Development|SetHiddeninGame (Variables|Default|GetTextRender) false false))

(event OnComponentEndOverlap(Box)
  (params (OverlappedComponent :type Primitive%20Component%20Object%20Reference) (OtherActor :type Actor%20Object%20Reference) (OtherComp :type Primitive%20Component%20Object%20Reference) (OtherBodyIndex :type Integer))
  ;[1 1 1] Texto sobre cofre
  (Utilities|Casting|CastToBP_MainCH OtherActor)
  (Development|SetHiddeninGame (Variables|Default|GetTextRender) true false))

(event EventBeginPlay)

(event Collision|EventActorBeginOverlap
  (params (OtherActor :type Actor%20Object%20Reference)))

(event EventTick
  (params (DeltaSeconds :type Float%20%28single-precision%29)))

(event EventInteract
  ;[1 1 1] Abrir/Cerrar cofre
  (if (Variables|Default|GetChestOpen)
    (Variables|Default|SetChestOpen false)
    (Components|Animation|PlayAnimation (Variables|Default|GetchestBox) "/Game/Model/chest/Assets/Chest_Anim_Armature_A_Close.Chest_Anim_Armature_A_Close" false)
    (else
      (Variables|Default|SetChestOpen true)
      (Components|Animation|PlayAnimation (Variables|Default|GetchestBox) "/Game/Model/chest/Assets/Chest_Anim_Armature_A_Open.Chest_Anim_Armature_A_Open" false))))

(fn ConstructionScript)